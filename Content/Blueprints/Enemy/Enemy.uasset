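; Enemy pawn that chases the player on sight and dies as a ragdoll on the first damage it takes.
; PawnSensing triggers AI MoveTo toward the seen ThirdPersonCharacterOld.
; Each tick turns the Plumbob widget horizontally toward the player camera, passes it the player's distance and calls its visibility toggle.
; AnyDamage and PointDamage share one death path: physics impulse from point-hit data, widget removal, capsule collision off, IsDed set.
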(event OnSeePawn(PawnSensing)
  (params (Pawn :type Pawn%20Object%20Reference))
  (bind _asthird_person_character_old (Utilities|Casting|CastToThirdPersonCharacterOld Pawn))
  (AI|AIMoveTo self (Transformation|GetActorLocation _asthird_person_character_old) _asthird_person_character_old 5.0 false))

(event Game|Damage|EventPointDamage
  (params (Damage :type Float%20%28single-precision%29) (DamageType :type Damage%20Type%20Object%20Reference) (HitLocation :type Vector) (HitNormal :type Vector) (HitComponent :type Primitive%20Component%20Object%20Reference) (BoneName :type Name) (ShotFromDirection :type Vector) (InstigatedBy :type Controller%20Object%20Reference) (DamageCauser :type Actor%20Object%20Reference) (HitInfo :type Hit%20Result%20Structure%20%28by%20ref%29))
  (bind _mesh (Variables|Character|GetMesh))
  (Physics|SetSimulatePhysics _mesh true)
  (Physics|AddImpulse _mesh (* (* HitLocation HitNormal) (/ Damage 1e+01)) "None" true)
  (Components|DestroyComponent (Variables|Default|GetWidget))
  (Collision|SetCollisionEnabled (Variables|Collision|GetCapsuleComponent) "NoCollision")
  (Variables|Default|SetisDed true))

(event EventTick
  (params (DeltaSeconds :type Float%20%28single-precision%29))
  (Transformation|SetWorldRotation (Variables|Default|GetWidget) (Math|Conversions|RotationFromXVector (Math|Vector|RotateVector (Math|Vector|Normalize (* (- (Transformation|GetWorldLocation (Variables|/Game/ThirdPersonBP/Blueprints/ThirdPersonCharacterOld.ThirdPersonCharacterOld_C|GetFollowCamera (.AsThird%20Person%20Character%20Old (Utilities|Casting|CastToThirdPersonCharacterOld (Game|GetPlayerCharacter 0))))) (Transformation|GetActorLocation)) "1.000000,1.000000, 0")) "0, 0, 0")) false false)
  (Variables|/Game/Widgets/Hud/Plumbob.Plumbob_C|SetDistance (Variables|Default|GetPlumbobRef) (Transformation|GetHorizontalDistanceTo (Game|Player|GetPlayerPawn 0)))
  (Default|ToggleVisibility (stale EventBeginPlay _output_get)))

(event EventBeginPlay
  (bind _asplumbob (Utilities|Casting|CastToPlumbob (UserInterface|GetUserWidgetObject (Variables|Default|GetWidget))))
  (bind _output_get (Variables|Default|SetPlumbobRef _asplumbob)))

(event Game|Damage|EventAnyDamage
  (params (Damage :type Float%20%28single-precision%29) (DamageType :type Damage%20Type%20Object%20Reference) (InstigatedBy :type Controller%20Object%20Reference) (DamageCauser :type Actor%20Object%20Reference))
  (bind _mesh (Variables|Character|GetMesh))
  (Physics|SetSimulatePhysics _mesh true)
  (Physics|AddImpulse _mesh (* (* (stale Game|Damage|EventPointDamage HitLocation) (stale Game|Damage|EventPointDamage HitNormal)) (/ (stale Game|Damage|EventPointDamage Damage) 1e+01)) "None" true)
  (Components|DestroyComponent (Variables|Default|GetWidget))
  (Collision|SetCollisionEnabled (Variables|Collision|GetCapsuleComponent) "NoCollision")
  (Variables|Default|SetisDed true))

(fn ConstructionScript)