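; Game Instance that holds and applies the interface's language, graphics and audio settings, loading defaults on first Init.
; Defaults select English, list supported resolutions and apply the desktop resolution.
; UpdateLanguage copies the language's data table into UIStructure, calls a forced language update and opens the Splash level.
; Graphics changes go through GameUserSettings and volumes through sound-mix class overrides; controls and gameplay updates are empty, and save-slot creation is unconnected.
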(event Custom|UpdateLanguage
  ;[1 1 1] Populate the LockedButtons array with the value from each row in the MissionTable data table.
  (switch Utilities|FlowControl|Switch|SwitchonLanguage_Language_Enum (Variables|Language|GetLanguage_Language)
    (:NewEnumerator0
      (Variables|System|SetDataTable "/Game/DataTables/UIData_English.UIData_English"))
    (:NewEnumerator1
      (Variables|System|SetDataTable "/Game/DataTables/UIData_French.UIData_French")))
  (bind _outrownames (DataTable|GetDataTableRowNames (Variables|System|GetDataTable)))
  (for _array_element _outrownames
    (bind _returnvalue (Utilities|GetDataTableRow (Variables|System|GetDataTable) _array_element)
      (:then
        (Utilities|Map|Add (Variables|System|GetUIStructure) _array_element _returnvalue))))
  (Default|CallForceLanguageUpdate)
  (Game|OpenLevel(byName) "Splash"))

(event Custom|UpdateGameplay)

(event Custom|UpdateControls)

(event Custom|LoadDefaultGameSettings
  (Utilities|FlowControl|Sequence
    (:then_0
      (Variables|Language|SetLanguage_Language "NewEnumerator0")
      (CallFunction|UpdateLanguage))
    (:then_1
      (bind _resolutions (Class|KismetSystemLibrary|GetSupportedFullscreenResolutions))
      (for _array_element _resolutions
        (Utilities|Array|Add (Variables|Graphics|GetGraphics_SupportedResolutions) (Utilities|ResolutiontoString (.x _array_element) (.y _array_element)))
        (bind _returnvalue (Settings|GetGameUserSettings))
        (CallFunction|SetScreenMode)
        (Class|GameUserSettings|SetScreenResolution _returnvalue (Class|GameUserSettings|GetDesktopResolution _returnvalue))
        (Class|GameUserSettings|ApplySettings _returnvalue false)
        (Variables|Graphics|SetGraphics_CurrentResolution (Utilities|ResolutiontoString (.x (Class|GameUserSettings|GetScreenResolution _returnvalue)) (.y (Class|GameUserSettings|GetScreenResolution _returnvalue))))))
    (:then_2
      (Settings|GetGameUserSettings))))

(event Custom|UpdateAudio
  ;[1 1 1] Update Audio
  (Utilities|FlowControl|Sequence
    (:then_0
      (Audio|SetSoundMixClassOverride "/Game/Audio/Master_Mix.Master_Mix" "/Game/Audio/Master_Class.Master_Class" (Variables|Audio|GetAudio_MasterVolume) 1.0 0.0 true))
    (:then_1
      (Audio|SetSoundMixClassOverride "/Game/Audio/Master_Mix.Master_Mix" "/Game/Audio/Music_Class.Music_Class" (Variables|Audio|GetAudio_MusicVolume) 1.0 0.0 true))
    (:then_2
      (Audio|SetSoundMixClassOverride "/Game/Audio/Master_Mix.Master_Mix" "/Game/Audio/Effects_Class.Effects_Class" (Variables|Audio|GetAudio_EffectsVolume) 1.0 0.0 true))
    (:then_3
      (Audio|SetSoundMixClassOverride "/Game/Audio/Master_Mix.Master_Mix" "/Game/Audio/Voice_Class.Voice_Class" (Variables|Audio|GetAudio_VoiceVolume) 1.0 0.0 true))))

(event Custom|UpdateGraphics
  (bind _returnvalue (Settings|GetGameUserSettings))
  (Class|GameUserSettings|ApplySettings _returnvalue false))

(event Custom|PushGraphicsSettings
  (bind _graphics_currentresolution (Variables|Graphics|GetGraphics_CurrentResolution))
  (bind (_resolutionx _resolutiony) (Utilities|StringtoResolution _graphics_currentresolution))
  (Utilities|FlowControl|Sequence
    (:then_0
      (bind _returnvalue (Settings|GetGameUserSettings))
      (Class|GameUserSettings|SetScreenResolution _returnvalue (Utilities|Struct|MakeIntPoint _resolutionx _resolutiony)))
    (:then_1
      (CallFunction|SetScreenMode))))

(event EventInit
  (if (Variables|System|GetFirstLoad)
    (Variables|System|SetFirstLoad false)
    (CallFunction|LoadDefaultGameSettings)))

(fn SetScreenMode
  (bind _returnvalue (Settings|GetGameUserSettings))
  (switch int (Variables|Graphics|GetGraphics_ScreenMode)
    (:0
      (Class|GameUserSettings|SetFullscreenMode _returnvalue "Fullscreen"))
    (:1
      (Class|GameUserSettings|SetFullscreenMode _returnvalue "Windowed"))
    (:2
      (Class|GameUserSettings|SetFullscreenMode _returnvalue "WindowedFullscreen"))))